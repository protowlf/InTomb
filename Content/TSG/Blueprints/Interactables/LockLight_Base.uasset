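; LockLight_Base is a light fixture that shows the glow color and active state of a referenced Interactable.
; The construction script creates one dynamic instance of M_TSGTransformingWorldMaterial, shared by both light meshes.
; BeginPlay applies the glow color to that material and both point lights, then binds to the Interactable's active-state change.
; Each change refreshes only the material color and switches both point lights on or off through intensity.
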(event Custom|OnActiveStateChanged
  (params (Interactable :type Interactable%20Base%20Object%20Reference) (IsActive :type Boolean))
  (Utilities|FlowControl|Sequence
    (:then_0
      (CallFunction|SetGlowColor (Default|GetGlowColor Interactable))
      (Rendering|Components|Light|SetIntensity (Variables|Default|GetPointLight1) (Math|Float|SelectFloat 1.5e+03 0.0 IsActive)))
    (:then_1)))

(event EventBeginPlay
  (bind _interactable (Variables|Default|GetInteractable))
  (bind _glowcolor (Default|GetGlowColor _interactable))
  (Utilities|IsValid _interactable
    (:Is%20Valid
      (CallFunction|SetGlowColor _glowcolor)
      (Rendering|Components|Light|SetLightColor (Variables|Default|GetPointLight1) _glowcolor true)
      (EventDispatchers|BindEventtoActiveStateChanged (Variables|Default|GetInteractable) (delegate Custom|OnActiveStateChanged)))))

(fn ConstructionScript
  (bind _returnvalue (Rendering|Material|CreateDynamicMaterialInstance (Variables|Default|GetLight1) 0 "/Game/TSG/Art/Materials/Shared/M_TSGTransformingWorldMaterial.M_TSGTransformingWorldMaterial" "None" :!class /Script/Engine.PrimitiveComponent))
  (bind _output_get (Variables|Default|SetGlowMaterial _returnvalue))
  (Rendering|Material|SetMaterial (Variables|Default|GetLight2) 0 _output_get))

(fn SetGlowColor
  (params (GlowColor :type Linear%20Color%20Structure))
  (Rendering|Material|SetVectorParameterValue (Variables|Default|GetGlowMaterial) "BaseColor" GlowColor :!class /Script/Engine.MaterialInstanceDynamic))