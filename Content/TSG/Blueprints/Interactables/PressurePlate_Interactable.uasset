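; Pressure plate interactable that sinks when triggered and fires the parent Interact logic once fully pressed.
; A timeline, rate-scaled by DepressTime, moves the Plate mesh on Z by DepressDistance, with Disabled set while it animates.
; Reset calls the parent and reverses the timeline, re-enabling the plate without firing Interact.
; Construction registers the Plate mesh through MakeMeshShowState; PressButton is only a debug print stub.
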(event EventBeginPlay
  (|CallParentFunction)
  (Variables|Internal|SetStartZ (.z (Variables|/Script/Engine.SceneComponent|GetRelativeLocation (Variables|Default|GetPlate))))
  (Components|Timeline|SetPlayRate (Variables|Default|GetButtonPressAnimation) (/ 1.0 (Variables|Default|GetDepressTime))))

(event EventTick
  (params (DeltaSeconds :type Float%20%28single-precision%29)))

(event EventInteract
  (Variables|Default|SetDisabled true)
  (bind (_direction _buttonz) (Timeline|ButtonPressAnimation Play)
    (:Update
      (Transformation|SetRelativeLocation (Variables|Default|GetPlate) (Math|Vector|MakeVector 0.0 0.0 (+ (Variables|Internal|GetStartZ) (* _buttonz (Variables|Default|GetDepressDistance)))) false false))
    (:Finished
      (Variables|Default|SetDisabled false)
      (if (Utilities|Enum|Equal(Enum) _direction "Forward")
        (|CallParentFunction)))))

(event EventReset
  (|CallParentFunction)
  (Variables|Default|SetDisabled true)
  (bind (_direction _buttonz) (Timeline|ButtonPressAnimation ReverseFromEnd)
    (:Update
      (Transformation|SetRelativeLocation (Variables|Default|GetPlate) (Math|Vector|MakeVector 0.0 0.0 (+ (Variables|Internal|GetStartZ) (* _buttonz (Variables|Default|GetDepressDistance)))) false false))
    (:Finished
      (Variables|Default|SetDisabled false)
      (if (Utilities|Enum|Equal(Enum) _direction "Forward")
        (|CallParentFunction)))))

(fn ConstructionScript
  (|CallParentFunction)
  (CallFunction|MakeMeshShowState (Variables|Default|GetPlate)))

(fn PressButton
  (Development|PrintString "Hello"))