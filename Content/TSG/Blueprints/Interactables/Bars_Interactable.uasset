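; Interactable set of bars that slides vertically to open when interacted with and slides back on reset.
; A timeline offsets the hinge's relative Z from its starting height, scaled by the door height.
; Play rate is set from separate open and close times, with Reset reversing the same timeline.
; It extends a parent interactable, and construction applies a show-state to the first mesh element.
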(event EventBeginPlay
  (|CallParentFunction)
  (Variables|Internal|SetStartLocationZ (.z (Variables|/Script/Engine.SceneComponent|GetRelativeLocation (Variables|Default|GetDoorHinge)))))

(event EventTick
  (params (DeltaSeconds :type Float%20%28single-precision%29))
  (|CallParentFunction DeltaSeconds) ; This node is disabled and will not be called.\nDrag off pins to build functionality.
)

(event EventReset
  (bind _doorhinge (Variables|Default|GetDoorHinge))
  (bind _relativelocation (Variables|/Script/Engine.SceneComponent|GetRelativeLocation _doorhinge))
  (|CallParentFunction)
  (Components|Timeline|SetPlayRate (Variables|Default|GetBarsSlideOpen) (/ 1.0 (Variables|Interactable|GetCloseTime)))
  (bind _hingez (Timeline|BarsSlideOpen Reverse)
    (:Update
      (Transformation|SetRelativeLocation _doorhinge (Math|Vector|MakeVector (.x _relativelocation) (.y _relativelocation) (+ (Variables|Internal|GetStartLocationZ) (* _hingez (Variables|Interactable|GetDoorHeight)))) false false))))

(event EventInteract
  (bind _doorhinge (Variables|Default|GetDoorHinge))
  (bind _relativelocation (Variables|/Script/Engine.SceneComponent|GetRelativeLocation _doorhinge))
  (|CallParentFunction)
  (Components|Timeline|SetPlayRate (Variables|Default|GetBarsSlideOpen) (/ 1.0 (Variables|Interactable|GetOpenTime)))
  (bind _hingez (Timeline|BarsSlideOpen Play)
    (:Update
      (Transformation|SetRelativeLocation _doorhinge (Math|Vector|MakeVector (.x _relativelocation) (.y _relativelocation) (+ (Variables|Internal|GetStartLocationZ) (* _hingez (Variables|Interactable|GetDoorHeight)))) false false))))

(fn ConstructionScript
  (|CallParentFunction)
  (CallFunction|MakeMeshShowState))