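; Player interaction component that tracks registered interactables and handles instant interactions, timed hold interactions and pickups.
; StartInteract drops any held pickup, otherwise selects an activatable target by a priority check (HighestPriority is never updated here).
; Holds slow the player's movement and aim while Tick feeds progress to the pawn, completing when full or cancelling on release.
; Pickups attach to PickupLocation with collision and physics off, and drop on entering ghost form.
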(event Custom|HoldToInteractSuccess
  (bind _currentholdtointeracttarget (Variables|Default|GetCurrentHoldToInteractTarget))
  (Utilities|FlowControl|Sequence
    (:then_0
      (Default|Interact _currentholdtointeracttarget)
      (if (Utilities|Enum|Equal(Enum) (Variables|/Game/TSG/Blueprints/Interactables/InteractableBase.InteractableBase_C|GetInteractableType _currentholdtointeracttarget) "NewEnumerator0")
        (CallFunction|PickUp _currentholdtointeracttarget)))
    (:then_1
      (CallFunction|EndHoldtoInteract true))))

(event EventBeginPlay)

(event EventTick
  (params (DeltaSeconds :type Float%20%28single-precision%29))
  (bind _returnvalue (Utilities|Time|GetTimeSeconds))
  (bind _holdtointeractstarttime (Variables|Default|GetHoldToInteractStartTime))
  (bind _holdtointeractduration (Variables|Default|GetHoldToInteractDuration))
  (bind _returnvalue_2 (- _returnvalue _holdtointeractstarttime))
  (bind _returnvalue_3 (/ _returnvalue_2 _holdtointeractduration))
  (bind _returnvalue_4 (Math|Float|Clamp(Float) _returnvalue_3))
  (if (Variables|Default|GetHoldToInteractActive)
    (Default|SetHoldtoInteractPercentage (CallFunction|GetTSGPlayerPawn) _returnvalue_4)
    (if (== _returnvalue_4 1.0)
      (CallFunction|HoldtoInteractSuccess))))

(event EventEnterGhostForm
  (params (EnteringInitialState :type Boolean))
  (Utilities|IsValid (Variables|Default|GetAttachedPickup)
    (:Is%20Valid
      (CallFunction|DropPickup self))))

(fn StartInteract
  (Utilities|IsValid (Variables|Default|GetAttachedPickup)
    (:Is%20Valid
      (CallFunction|DropPickup self))
    (:Is%20Not%20Valid
      (bind (_foundinteractable _bestinteractable) (CallFunction|FindBestInteractable))
      (if _foundinteractable
        (if (Variables|/Game/TSG/Blueprints/Interactables/InteractableBase.InteractableBase_C|GetHoldToInteract _bestinteractable)
          (CallFunction|StartHoldtoInteract _bestinteractable)
          (else
            (Default|Interact _bestinteractable)
            (if (Utilities|Enum|Equal(Enum) (Variables|/Game/TSG/Blueprints/Interactables/InteractableBase.InteractableBase_C|GetInteractableType _bestinteractable) "NewEnumerator0")
              (CallFunction|PickUp _bestinteractable))))))))

(fn EndInteract
  (if (Variables|Default|GetHoldToInteractActive)
    (CallFunction|EndHoldtoInteract false)))

(fn FindBestInteractable
  (for _array_element (Variables|Default|GetInteractables)
    (if (Default|CanActivate _array_element)
      (if (>= (Variables|/Game/TSG/Blueprints/Interactables/InteractableBase.InteractableBase_C|GetPriority _array_element) (LocalVariables|GetHighestPriority))
        (LocalVariables|SetBestInteractble _array_element))))
  (Utilities|IsValid (LocalVariables|GetBestInteractble)
    (:Is%20Valid
      (return true (LocalVariables|GetBestInteractble)))
    (:Is%20Not%20Valid
      (return false 0))))

(fn AddInteractable
  (params (Interactable :type Interactable%20Base%20Object%20Reference%20%28by%20ref%29))
  (Utilities|IsValid Interactable
    (:Is%20Valid
      (bind _returnvalue (Utilities|Array|AddUnique (Variables|Default|GetInteractables) Interactable))
      (Utilities|FlowControl|Sequence
        (:then_0
          (if (and (Variables|Default|GetDebugInteract) (>= _returnvalue 0))
            (Development|PrintString (Utilities|String|Append "ADDED " (Utilities|GetDisplayName Interactable)) true true "(R=0.139614,G=1.000000,B=0.000000,A=1.000000)")))
        (:then_1
          (return (>= _returnvalue 0)))))))

(fn RemoveInteractable
  (params (Interactable :type Interactable%20Base%20Object%20Reference%20%28by%20ref%29))
  (Utilities|IsValid Interactable
    (:Is%20Valid
      (bind _returnvalue (Utilities|Array|RemoveItem (Variables|Default|GetInteractables) Interactable))
      (Utilities|FlowControl|Sequence
        (:then_0
          (if (and (Variables|Default|GetDebugInteract) _returnvalue)
            (Development|PrintString (Utilities|String|Append "REMOVED " (Utilities|GetDisplayName Interactable)) true true "(R=1.000000,G=0.000000,B=0.136240,A=1.000000)")))
        (:then_1
          (return _returnvalue))))))

(fn PickUp
  (params (PickUp :type Interactable%20Base%20Object%20Reference))
  (Collision|SetActorEnableCollision PickUp false)
  (Physics|SetSimulatePhysics (Variables|/Game/TSG/Blueprints/Interactables/InteractableBase.InteractableBase_C|GetMeshRoot PickUp) false)
  (Transformation|AttachComponentToComponent PickUp (Variables|Default|GetPickupLocation) "None" "SnapToTarget" "SnapToTarget" "KeepRelative" true)
  (Variables|Default|SetAttachedPickup PickUp))

(fn DropPickup
  (Transformation|DetachFromActor (Variables|Default|GetAttachedPickup) "KeepWorld" "KeepWorld" "KeepRelative")
  (Collision|SetActorEnableCollision (Variables|Default|GetAttachedPickup) true)
  (Physics|SetSimulatePhysics (Variables|/Game/TSG/Blueprints/Interactables/InteractableBase.InteractableBase_C|GetMeshRoot (Variables|Default|GetAttachedPickup)) true)
  (Variables|Default|SetAttachedPickup 0))

(fn StartHoldtoInteract
  (params (HoldToInteractTarget :type Interactable%20Base%20Object%20Reference))
  (Utilities|FlowControl|Sequence
    (:then_0
      (Variables|Default|SetHoldToInteractActive true)
      (bind _output_get (Variables|Default|SetCurrentHoldToInteractTarget HoldToInteractTarget))
      (Variables|Default|SetHoldToInteractDuration (Variables|/Game/TSG/Blueprints/Interactables/InteractableBase.InteractableBase_C|GetHoldToInteractTime _output_get))
      (Variables|Default|SetHoldToInteractStartTime (Utilities|Time|GetTimeSeconds)))
    (:then_1
      (Default|SetMoveandAimSpeedScalar (CallFunction|GetTSGPlayerPawn) 0.2 0.2))
    (:then_2
      (Default|StartHoldtoInteract HoldToInteractTarget))))

(fn EndHoldtoInteract
  (params (Success :type Boolean))
  (bind _astsgplayer_pawn (CallFunction|GetTSGPlayerPawn))
  (Utilities|FlowControl|Sequence
    (:then_0
      (Default|EndHoldtoInteract (Variables|Default|GetCurrentHoldToInteractTarget) Success))
    (:then_1
      (Variables|Default|SetHoldToInteractActive false)
      (Variables|Default|SetCurrentHoldToInteractTarget 0))
    (:then_2
      (Default|SetMoveandAimSpeedScalar _astsgplayer_pawn 1.0 1.0)
      (Default|SetHoldtoInteractPercentage _astsgplayer_pawn 0.0))))