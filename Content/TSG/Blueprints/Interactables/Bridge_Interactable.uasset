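; Interactable bridge that starts lowered, rises when interacted with and sinks back on reset.
; BeginPlay drops the bridge by the lift distance from its placed position and stores that Z as the start height.
; Interact plays the LiftBridge timeline, whose HingeZ track scales the lift distance to drive the bridge's relative Z.
; Reset reverses the same timeline, with play rates derived from separate lift and fall times.
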(event EventBeginPlay
  (bind _fullbridge (Variables|Default|GetFullBridge))
  (bind _relativelocation (Variables|/Script/Engine.SceneComponent|GetRelativeLocation _fullbridge))
  (|CallParentFunction)
  (Transformation|SetRelativeLocation _fullbridge (Math|Vector|MakeVector (.x _relativelocation) (.y _relativelocation) (- (.z _relativelocation) (Variables|Interactable|GetBridgeLiftDistance))) false true)
  (Variables|Internal|SetStartLocationZ (.z _relativelocation)))

(event EventReset
  (bind _fullbridge (Variables|Default|GetFullBridge))
  (bind _relativelocation (Variables|/Script/Engine.SceneComponent|GetRelativeLocation _fullbridge))
  (|CallParentFunction)
  (Components|Timeline|SetPlayRate (Variables|Default|GetLiftBridge) (/ 1.0 (Variables|Interactable|GetFallTime)))
  (bind _hingez (Timeline|LiftBridge Reverse)
    (:Update
      (Transformation|SetRelativeLocation _fullbridge (Math|Vector|MakeVector (.x _relativelocation) (.y _relativelocation) (+ (Variables|Internal|GetStartLocationZ) (* _hingez (Variables|Interactable|GetBridgeLiftDistance)))) false false))))

(event EventInteract
  (bind _fullbridge (Variables|Default|GetFullBridge))
  (bind _relativelocation (Variables|/Script/Engine.SceneComponent|GetRelativeLocation _fullbridge))
  (|CallParentFunction)
  (Components|Timeline|SetPlayRate (Variables|Default|GetLiftBridge) (/ 1.0 (Variables|Interactable|GetLiftTime)))
  (bind _hingez (Timeline|LiftBridge Play)
    (:Update
      (Transformation|SetRelativeLocation _fullbridge (Math|Vector|MakeVector (.x _relativelocation) (.y _relativelocation) (+ (Variables|Internal|GetStartLocationZ) (* _hingez (Variables|Interactable|GetBridgeLiftDistance)))) false false))))

(fn ConstructionScript
  (|CallParentFunction))