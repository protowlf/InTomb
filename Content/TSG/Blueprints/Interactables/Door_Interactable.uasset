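; Interactable door Blueprint that opens on Interact and closes on Reset, either swinging around its hinge or sliding vertically.
; A single timeline drives hinge yaw or height from the starting transform, playing forward or reversed with separate open and close durations.
; Door collision turns off when opening starts and returns only after closing finishes.
; A camera shake source runs during movement and stops when the timeline finishes.
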(event EventBeginPlay
  (bind _doorhinge (Variables|Default|GetDoorHinge))
  (|CallParentFunction)
  (Variables|Internal|SetStartRotationZ (.yaw (Variables|/Script/Engine.SceneComponent|GetRelativeRotation _doorhinge)))
  (Variables|Internal|SetStartLocationZ (.z (Variables|/Script/Engine.SceneComponent|GetRelativeLocation _doorhinge)))
  (Components|Timeline|SetPlayRate (Variables|Default|GetDoorSwingOpen) (/ 1.0 (Variables|Interactable|GetOpenTime))))

(event EventReset
  (bind _doorhinge (Variables|Default|GetDoorHinge))
  (bind _openangle (Variables|Interactable|GetOpenAngle))
  (bind _relativelocation (Variables|/Script/Engine.SceneComponent|GetRelativeLocation _doorhinge))
  (|CallParentFunction)
  (CameraShake|Start (Variables|Default|GetCameraShakeSource))
  (Components|Timeline|SetPlayRate (Variables|Default|GetDoorSwingOpen) (/ 1.0 (Variables|Interactable|GetCloseTime)))
  (bind (_direction _hingez) (Timeline|DoorSwingOpen Reverse)
    (:Update
      (if (Variables|Interactable|GetSlidingDoor)
        (Transformation|SetRelativeLocation _doorhinge (Math|Vector|MakeVector (.x _relativelocation) (.y _relativelocation) (+ (Variables|Internal|GetStartLocationZ) (* _hingez (Variables|Interactable|GetDoorHeight)))) false false)
        (else
          (Transformation|SetRelativeRotation (Variables|Default|GetDoorHinge) (Math|Rotator|MakeRotator 0.0 0.0 (+ (Variables|Internal|GetStartRotationZ) (* _hingez (select (Variables|Interactable|GetOpensOtherWay) (* _openangle -1.0) _openangle)))) false false))))
    (:Finished
      (CameraShake|StopAllCameraShakes (Variables|Default|GetCameraShakeSource) true)
      (if (Utilities|Enum|Equal(Enum) _direction "Backward")
        (Collision|SetCollisionEnabled (Variables|Default|GetDoor) "QueryAndPhysics")))))

(event EventInteract
  (bind _doorhinge (Variables|Default|GetDoorHinge))
  (bind _openangle (Variables|Interactable|GetOpenAngle))
  (bind _relativelocation (Variables|/Script/Engine.SceneComponent|GetRelativeLocation _doorhinge))
  (|CallParentFunction)
  (CameraShake|Start (Variables|Default|GetCameraShakeSource))
  (Collision|SetCollisionEnabled (Variables|Default|GetDoor) "NoCollision")
  (Components|Timeline|SetPlayRate (Variables|Default|GetDoorSwingOpen) (/ 1.0 (Variables|Interactable|GetOpenTime)))
  (bind (_direction _hingez) (Timeline|DoorSwingOpen Play)
    (:Update
      (if (Variables|Interactable|GetSlidingDoor)
        (Transformation|SetRelativeLocation _doorhinge (Math|Vector|MakeVector (.x _relativelocation) (.y _relativelocation) (+ (Variables|Internal|GetStartLocationZ) (* _hingez (Variables|Interactable|GetDoorHeight)))) false false)
        (else
          (Transformation|SetRelativeRotation (Variables|Default|GetDoorHinge) (Math|Rotator|MakeRotator 0.0 0.0 (+ (Variables|Internal|GetStartRotationZ) (* _hingez (select (Variables|Interactable|GetOpensOtherWay) (* _openangle -1.0) _openangle)))) false false))))
    (:Finished
      (CameraShake|StopAllCameraShakes (Variables|Default|GetCameraShakeSource) true)
      (if (Utilities|Enum|Equal(Enum) _direction "Backward")
        (Collision|SetCollisionEnabled (Variables|Default|GetDoor) "QueryAndPhysics")))))

(fn ConstructionScript
  (|CallParentFunction)
  (CallFunction|MakeMeshShowState (Variables|Default|GetActiveState)))