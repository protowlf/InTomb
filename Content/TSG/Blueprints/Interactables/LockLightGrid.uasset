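; Lock light grid that shows the keys of its parent InteractableBase actor as a row of indicator lights.
; The construction script caches the parent, and BeginPlay spawns one LockLight_Base per key, spaced by GridGap around a fixed offset from the root.
; The row runs along world Y regardless of the root's rotation.
; Tick copies each key's glow color onto the light with the same index.
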(event EventBeginPlay
  (bind _interactable (Variables|Default|GetInteractable))
  (bind _defaultsceneroot (Variables|Default|GetDefaultSceneRoot))
  (bind _returnvalue (Transformation|GetWorldLocation _defaultsceneroot))
  (bind _keys (Variables|/Game/TSG/Blueprints/Interactables/InteractableBase.InteractableBase_C|GetKeys _interactable))
  (for (_array_element _array_index) _keys
    (bind _returnvalue_2 (Game|SpawnActorfromClass "/Game/TSG/Blueprints/Interactables/LockLight_Base.LockLight_Base_C" (Math|Transform|MakeTransform (Math|Vector|MakeVector (.x _returnvalue) (+ (.y _returnvalue) (Math|Conversions|ToFloat(Integer) (* (Variables|Default|GetGridGap) _array_index)) (* (Math|Conversions|ToFloat(Integer) (* (Math|Integer|Max(Integer) (- (Utilities|Array|Length _keys) 1)) (Variables|Default|GetGridGap))) -0.5) 53.0) (.z _returnvalue)) (Transformation|GetWorldRotation _defaultsceneroot) (Transformation|GetWorldScale _defaultsceneroot)) "AlwaysSpawn" self _array_element 0))
    (Utilities|IsValid _returnvalue_2
      (:Is%20Valid
        (Utilities|Array|Add (Variables|Default|GetLockLights) _returnvalue_2)))))

(event EventTick
  (params (DeltaSeconds :type Float%20%28single-precision%29))
  (for (_array_element _array_index) (Variables|/Game/TSG/Blueprints/Interactables/InteractableBase.InteractableBase_C|GetKeys (Variables|Default|GetInteractable))
    (Default|SetGlowColor (Utilities|Array|Get(acopy) (Variables|Default|GetLockLights) _array_index) (Default|GetGlowColor _array_element))))

(fn ConstructionScript
  (CallFunction|Init))

(fn Init
  (bind _asinteractable_base (Utilities|Casting|CastToInteractableBase (Actor|GetParentActor)))
  (Variables|Default|SetInteractable _asinteractable_base))