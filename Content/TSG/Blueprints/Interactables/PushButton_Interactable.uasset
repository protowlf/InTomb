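; Push button interactable that animates its button mesh pressing in when used and extending back out on reset.
; A timeline, rate-scaled by DepressTime, offsets the button's relative Z by DepressDistance from its starting height.
; The parent Interact is deferred until the forward press finishes, while Reset calls the parent and plays the timeline in reverse.
; Hold-to-interact events are empty, and PressButton only prints debug text.
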(event EventBeginPlay
  (|CallParentFunction)
  (Variables|Internal|SetStartZ (.z (Variables|/Script/Engine.SceneComponent|GetRelativeLocation (Variables|Default|GetButton))))
  (Components|Timeline|SetPlayRate (Variables|Default|GetButtonPressAnimation) (/ 1.0 (Variables|Default|GetDepressTime))))

(event EventStartHoldtoInteract)

(event EventInteract
  (bind _button (Variables|Default|GetButton))
  (bind _relativelocation (Variables|/Script/Engine.SceneComponent|GetRelativeLocation _button))
  (bind (_direction _buttonz) (Timeline|ButtonPressAnimation Play)
    (:Update
      (Transformation|SetRelativeLocation _button (Math|Vector|MakeVector (.x _relativelocation) (.y _relativelocation) (+ (Variables|Internal|GetStartZ) (* _buttonz (Variables|Default|GetDepressDistance)))) false false))
    (:Finished
      (if (Utilities|Enum|Equal(Enum) _direction "Forward")
        (|CallParentFunction)))))

(event EventReset
  (bind _button (Variables|Default|GetButton))
  (bind _relativelocation (Variables|/Script/Engine.SceneComponent|GetRelativeLocation _button))
  (|CallParentFunction)
  (bind (_direction _buttonz) (Timeline|ButtonPressAnimation ReverseFromEnd)
    (:Update
      (Transformation|SetRelativeLocation _button (Math|Vector|MakeVector (.x _relativelocation) (.y _relativelocation) (+ (Variables|Internal|GetStartZ) (* _buttonz (Variables|Default|GetDepressDistance)))) false false))
    (:Finished
      (if (Utilities|Enum|Equal(Enum) _direction "Forward")
        (|CallParentFunction)))))

(event EventEndHoldtoInteractEarly)

(fn ConstructionScript
  (|CallParentFunction)
  (CallFunction|MakeMeshShowState (Variables|Default|GetButton)))

(fn PressButton
  (Development|PrintString "Hello"))