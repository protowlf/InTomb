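; Game mode that manages the player's switch between ghost and mortal form, with mortal form lasting a limited time.
; PlayerTryEnterMortalForm starts mortal form if not already active, and Tick runs a countdown that returns the player to ghost form when it expires.
; Each switch notifies every I_TSGGameObject actor and starts a timed blend of MortalFormPercent in the TSGWorldMaterialParameters collection, driving a world-wide material transition.
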(event EventBeginPlay)

(event EventTick
  (params (DeltaSeconds :type Float%20%28single-precision%29))
  (Utilities|FlowControl|Sequence
    (:then_0
      (if (Variables|Default|GetIsMortalForm)
        (Protected|UpdateMortalFormCountdown)))
    (:then_1
      (if (Variables|MortalFormMaterialTransition|GetIsMFMTActive_ToMortal)
        (Protected|UpdateMFMTtoMortal)))
    (:then_2
      (if (Variables|MortalFormMaterialTransition|GetIsMFMTActive_ToGhost)
        (Protected|UpdateMFMTtoGhost)))))

(fn ConstructionScript)

(fn PlayerTryEnterMortalForm
  (if (not (Variables|Default|GetIsMortalForm))
    (Protected|PlayerEnterMortalForm)
    (return true)
    (else
      (return false))))

(fn PlayerEnterMortalForm
  (Utilities|FlowControl|Sequence
    (:then_0
      (Variables|Default|SetIsMortalForm true)
      (Variables|Default|SetMortalFormStartTime (Utilities|Time|GetTimeSeconds)))
    (:then_1
      ;[1 1 1] Send event to TSG Game Objects
      (bind _outactors (Actor|GetAllActorswithInterface "/Game/TSG/Blueprints/Core/I_TSGGameObject.I_TSGGameObject_C"))
      (for _array_element _outactors
        (bind _asi_tsggame_object (Utilities|Casting|CastToI_TSGGameObject _array_element))
        (Default|EnterMortalForm _asi_tsggame_object)))
    (:then_2
      (Variables|MortalFormMaterialTransition|SetIsMFMTActive_ToMortal true)
      (Variables|MortalFormMaterialTransition|SetMFMTStartTime (Utilities|Time|GetTimeSeconds)))))

(fn UpdateMFMTtoMortal
  (bind _output_get (LocalVariables|SetPercentageEllapsed (Math|Float|Clamp(Float) (/ (- (Utilities|Time|GetTimeSeconds) (Variables|MortalFormMaterialTransition|GetMFMTStartTime)) (Variables|MortalFormMaterialTransition|GetMFMTDuration)))))
  (Rendering|Material|SetScalarParameterValue "/Game/TSG/Art/Materials/Shared/TSGWorldMaterialParameters.TSGWorldMaterialParameters" "MortalFormPercent" _output_get :!class /Script/Engine.KismetMaterialLibrary)
  (if (== (LocalVariables|GetPercentageEllapsed) 1.0)
    (Variables|MortalFormMaterialTransition|SetIsMFMTActive_ToMortal false)))

(fn UpdateMFMTtoGhost
  (bind _output_get (LocalVariables|SetPercentageEllapsed (Math|Float|Clamp(Float) (/ (- (Utilities|Time|GetTimeSeconds) (Variables|MortalFormMaterialTransition|GetMFMTStartTime)) (Variables|MortalFormMaterialTransition|GetMFMTDuration)))))
  (Rendering|Material|SetScalarParameterValue "/Game/TSG/Art/Materials/Shared/TSGWorldMaterialParameters.TSGWorldMaterialParameters" "MortalFormPercent" (- 1.0 _output_get) :!class /Script/Engine.KismetMaterialLibrary)
  (if (== (LocalVariables|GetPercentageEllapsed) 1.0)
    (Variables|MortalFormMaterialTransition|SetIsMFMTActive_ToGhost false)))

(fn UpdateMortalFormCountdown
  (Utilities|FlowControl|Sequence
    (:then_0
      ;[1 1 1] Comment
      (LocalVariables|SetPercentageEllapsed (Math|Float|Clamp(Float) (/ (- (Utilities|Time|GetTimeSeconds) (Variables|Default|GetMortalFormStartTime)) (Variables|Default|GetMortalFormDuration)))))
    (:then_1
      (if (== (LocalVariables|GetPercentageEllapsed) 1.0)
        (Protected|PlayerEnterGhostForm)))))

(fn PlayerEnterGhostForm
  (Utilities|FlowControl|Sequence
    (:then_0
      (Variables|Default|SetIsMortalForm false))
    (:then_1
      ;[1 1 1] Send event to TSG Game Objects
      (bind _outactors (Actor|GetAllActorswithInterface "/Game/TSG/Blueprints/Core/I_TSGGameObject.I_TSGGameObject_C"))
      (for _array_element _outactors
        (bind _asi_tsggame_object (Utilities|Casting|CastToI_TSGGameObject _array_element))
        (Default|EnterGhostForm _asi_tsggame_object)))
    (:then_2
      (Variables|MortalFormMaterialTransition|SetIsMFMTActive_ToGhost true)
      (Variables|MortalFormMaterialTransition|SetMFMTStartTime (Utilities|Time|GetTimeSeconds)))))

(fn IsPlayerMortalForm
  (return (Variables|Default|GetIsMortalForm)))