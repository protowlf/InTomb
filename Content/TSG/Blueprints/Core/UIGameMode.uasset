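; UI game mode that shows the mouse cursor on BeginPlay and carries what looks like stubbed ghost/mortal form switching logic.
; The enter-form functions broadcast to every actor implementing I_TSGGameObject, and initial ghost entry sets the GhostFormPercent material collection parameter.
; Transition and countdown helpers use hard-coded timings and are not called here, as Tick is empty.
; The mortal-form query always returns false.
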(event EventBeginPlay
  (Variables|/Script/Engine.PlayerController|SetbShowMouseCursor (Game|GetPlayerController 0) true))

(event EventTick
  (params (DeltaSeconds :type Float%20%28single-precision%29)))

(fn ConstructionScript)

(fn PlayerTryEnterMortalForm
  (if (not false)
    (Protected|PlayerEnterMortalForm)
    (return true)
    (else
      (return false))))

(fn PlayerEnterMortalForm
  (Utilities|FlowControl|Sequence
    (:then_1
      ;[1 1 1] Send event to TSG Game Objects
      (bind _outactors (Actor|GetAllActorswithInterface "/Game/TSG/Blueprints/Core/I_TSGGameObject.I_TSGGameObject_C"))
      (for _array_element _outactors
        (bind _asi_tsggame_object (Utilities|Casting|CastToI_TSGGameObject _array_element))
        (Default|EnterMortalForm _asi_tsggame_object)))))

(fn UpdateMFMTtoMortal
  (bind _output_get (LocalVariables|SetPercentageEllapsed (Math|Float|Clamp(Float) (/ (- (Utilities|Time|GetTimeSeconds) 1.0) 1.0))))
  (Rendering|Material|SetScalarParameterValue "/Game/TSG/Art/Materials/Shared/TSGWorldMaterialParameters.TSGWorldMaterialParameters" "GhostFormPercent" (- 1.0 _output_get) :!class /Script/Engine.KismetMaterialLibrary)
  (if (== (LocalVariables|GetPercentageEllapsed) 1.0)
    _))

(fn UpdateMFMTtoGhost
  (bind _output_get (LocalVariables|SetPercentageEllapsed (Math|Float|Clamp(Float) (/ (- (Utilities|Time|GetTimeSeconds) 1.0) 1.0))))
  (Rendering|Material|SetScalarParameterValue "/Game/TSG/Art/Materials/Shared/TSGWorldMaterialParameters.TSGWorldMaterialParameters" "GhostFormPercent" _output_get :!class /Script/Engine.KismetMaterialLibrary)
  (if (== (LocalVariables|GetPercentageEllapsed) 1.0)
    _))

(fn UpdateMortalFormCountdown
  (Utilities|FlowControl|Sequence
    (:then_0
      ;[1 1 1] Comment
      (LocalVariables|SetPercentageEllapsed (Math|Float|Clamp(Float) (/ (- (Utilities|Time|GetTimeSeconds) 1.0) 1.0))))
    (:then_1
      (if (== (LocalVariables|GetPercentageEllapsed) 1.0)
        (Protected|PlayerEnterGhostForm false)))))

(fn PlayerEnterGhostForm
  (params (EnteringInitialState :type Boolean))
  (Utilities|FlowControl|Sequence
    (:then_1
      ;[1 1 1] Send event to TSG Game Objects
      (bind _outactors (Actor|GetAllActorswithInterface "/Game/TSG/Blueprints/Core/I_TSGGameObject.I_TSGGameObject_C"))
      (for _array_element _outactors
        (bind _asi_tsggame_object (Utilities|Casting|CastToI_TSGGameObject _array_element))
        (Default|EnterGhostForm _asi_tsggame_object EnteringInitialState)))
    (:then_2
      (if EnteringInitialState
        (Rendering|Material|SetScalarParameterValue "/Game/TSG/Art/Materials/Shared/TSGWorldMaterialParameters.TSGWorldMaterialParameters" "GhostFormPercent" 1.0 :!class /Script/Engine.KismetMaterialLibrary)))))

(fn IsPlayerMortalForm
  (return false))