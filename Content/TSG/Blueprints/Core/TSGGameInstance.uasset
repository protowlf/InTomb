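; Game instance Blueprint that handles progression from the current level to the next.
; GoToNextLevel scans the LevelTransitions DataTable for the row matching the current level name and passes its NextLevel to LevelTransition, printing an error if none matches.
; LevelTransition fades the player camera and audio out, waits through the fade and hold times, then opens the level by name.
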(event Custom|LevelTransition
  (params (NextLevelName :type Name))
  (CameraFades|StartCameraFade :self (Variables|/Script/Engine.PlayerController|GetPlayerCameraManager (Game|GetPlayerController 0)) :ToAlpha 1.0 :Duration (Variables|Default|GetLevelTransitionFadeDownTime) :bShouldFadeAudio true :bHoldWhenFinished true)
  (Utilities|FlowControl|Delay (+ (Variables|Default|GetLevelTransitionFadeDownTime) (Variables|Default|GetLevelTransitionFadeHoldTime)))
  (Game|OpenLevel(byName) NextLevelName))

(fn GotoNextLevel
  (bind _leveltransitionsdatatable (Variables|Default|GetLevelTransitionsDataTable))
  (bind _outrownames (DataTable|GetDataTableRowNames _leveltransitionsdatatable))
  (for _array_element _outrownames
    (bind _returnvalue (Utilities|GetDataTableRow _leveltransitionsdatatable _array_element)
      (:then
        (bind _returnvalue_2 (Game|GetCurrentLevelName true))
        (if (Utilities|Enum|Equal(Enum) _returnvalue_2 (Utilities|String|ToString(Name) (.LevelName (Utilities|Struct|BreakLevelTransitionData _returnvalue))))
          (LocalVariables|SetFoundLevelData true)
          (LocalVariables|SetNextLevel (.NextLevel (Utilities|Struct|BreakLevelTransitionData _returnvalue)))))))
  (if (LocalVariables|GetFoundLevelData)
    (CallFunction|LevelTransition (LocalVariables|GetNextLevel))
    (else
      (Development|PrintString "GoToNextLevel couldn't find data for the next level! Check LevelTransitions DataTable" true true "(R=1.000000,G=0.000000,B=0.057227,A=1.000000)"))))