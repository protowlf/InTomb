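; Player view model that shows the right hand and swaps its pose between Ghost and Mortal forms.
; Form events toggle visibility between the normal hand and the mortal-pose hand, with entering Mortal form also spawning an attached spell effect at MortalSpellLoc.
; An AllowMortalFormSpell flag hides the normal hand at BeginPlay when off, and SetAllowMortalForm updates the flag and that hand's visibility.
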(event EventBeginPlay
  (if (not (Variables|Default|GetAllowMortalFormSpell))
    (Rendering|SetVisibility (Variables|Default|GetTSGHand_Right) false false)))

(event Collision|EventActorBeginOverlap
  (params (OtherActor :type Actor%20Object%20Reference)))

(event EventTick
  (params (DeltaSeconds :type Float%20%28single-precision%29)))

(event EventEnterGhostForm
  (params (EnteringInitialState :type Boolean))
  (Rendering|SetVisibility (Variables|Default|GetTSGHand_Right) true false)
  (Rendering|SetVisibility (Variables|Default|GetTSGHand_RightMortalPose) false false))

(event EventEnterMortalForm
  (Niagara|SpawnSystemAttached "/Game/TSG/Art/Particles/PlayerMortalSpell.PlayerMortalSpell" (Variables|Default|GetMortalSpellLoc) "None" "0, 0, 0" "0, 0, 0" "KeepRelativeOffset" false)
  (Rendering|SetVisibility (Variables|Default|GetTSGHand_Right) false false)
  (Rendering|SetVisibility (Variables|Default|GetTSGHand_RightMortalPose) true false))

(fn ConstructionScript)

(fn SetAllowMortalForm
  (params (Bool :type Boolean))
  (bind _output_get (Variables|Default|SetAllowMortalFormSpell Bool))
  (if _output_get
    (Rendering|SetVisibility (Variables|Default|GetTSGHand_Right) true false)
    (else
      (Rendering|SetVisibility (Variables|Default|GetTSGHand_Right) false false))))