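; TSGPlayerFX is a player effects component that handles visual and audio feedback for switching between ghost and mortal forms.
; Entering ghost form spawns a vignette Niagara system attached to itself and a 2D whisper sound, storing both instances.
; Entering mortal form destroys those stored instances and plays a one-shot 2D whoosh.
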(event EventBeginPlay)

(event EventTick
  (params (DeltaSeconds :type Float%20%28single-precision%29)))

(event EventEnterGhostForm
  (params (EnteringInitialState :type Boolean))
  (Utilities|FlowControl|Sequence
    (:then_0
      (bind _returnvalue (Niagara|SpawnSystemAttached (Variables|Default|GetVFX_GhostFormVignette) self "None" "0, 0, 0" "0, 0, 0" "KeepRelativeOffset" false))
      (Variables|Default|SetVFXInst_GhostFormVignete _returnvalue))
    (:then_1
      (bind _returnvalue_2 (Audio|SpawnSound2D (Variables|Default|GetGhostFormWhispers) 1.0 1.0 0.0 0))
      (Variables|Default|SetInst_GhostFormWhispers _returnvalue_2))))

(event EventEnterMortalForm
  (Utilities|FlowControl|Sequence
    (:then_0
      (Components|DestroyComponent (Variables|Default|GetVFXInst_GhostFormVignete))
      (Components|DestroyComponent (Variables|Default|GetInst_GhostFormWhispers)))
    (:then_1
      (Audio|PlaySound2D "/Game/TSG/Sound/EnterMortalFormWoosh.EnterMortalFormWoosh" 1.0 1.0 0.0 0 0))))