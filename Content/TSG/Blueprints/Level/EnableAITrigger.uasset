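; Level trigger actor that enables or disables movement for a set of assigned AI when the player overlaps it.
; On overlap by the TSG player pawn, it calls AllowMovement with the SetEnabled flag on each valid entry in its AI array.
; Unless TriggerMultiple is set, it destroys itself after firing, making it a one-shot trigger.
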(event Collision|EventActorBeginOverlap
  (params (OtherActor :type Actor%20Object%20Reference))
  (if (== OtherActor (CallFunction|GetTSGPlayerPawn))
    (for _array_element (Variables|Default|GetAI)
      (Utilities|IsValid _array_element
        (:Is%20Valid
          (Default|AllowMovement _array_element (Variables|Default|GetSetEnabled)))))
    (if (not (Variables|Default|GetTriggerMultiple))
      (Actor|DestroyActor self))))

(fn ConstructionScript)