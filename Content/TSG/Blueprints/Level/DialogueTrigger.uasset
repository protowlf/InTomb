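; DialogueTrigger is a level-placed trigger actor that shows subtitle dialogue on the HUD when the TSG player pawn overlaps it.
; It passes its passage text and post-print display time to the pawn's DisplaySubtitlesOnHud function.
; Unless TriggerMultiple is set, it destroys itself after the first trigger.
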(event Collision|EventActorBeginOverlap
  (params (OtherActor :type Actor%20Object%20Reference))
  (bind _astsgplayer_pawn (CallFunction|GetTSGPlayerPawn))
  (if (== OtherActor _astsgplayer_pawn)
    (Default|DisplaySubtitlesonHud _astsgplayer_pawn (Variables|Default|GetPassageText) (Variables|Default|GetTimeAfterFinishingPrint))
    (if (not (Variables|Default|GetTriggerMultiple))
      (Actor|DestroyActor self))))

(fn ConstructionScript)