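; GuardA is an enemy guard that switches between a wandering ghost form and a lethal mortal form.
; Each form swaps the visible body and movement tuning, and ghost form starts on BeginPlay.
; As a ghost it records its location as home, then uses randomized timers for AI moves to reachable points nearby.
; As a mortal it chases the player every Tick unless movement is disabled, and kills them on capsule overlap.
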(event OnComponentBeginOverlap(CapsuleComponent)
  (params (OverlappedComponent :type Primitive%20Component%20Object%20Reference) (OtherActor :type Actor%20Object%20Reference) (OtherComp :type Primitive%20Component%20Object%20Reference) (OtherBodyIndex :type Integer) (bFromSweep :type Boolean) (SweepResult :type Hit%20Result%20Structure%20%28by%20ref%29))
  (if (Variables|Default|GetIsMortalForm)
    (bind _astsgplayer_pawn (Utilities|Casting|CastToTSGPlayerPawn OtherActor))
    (Default|EventDie _astsgplayer_pawn)))

(event Custom|GhostFormMoveEvent
  (AI|AIMoveTo self (.RandomLocation (AI|Navigation|GetRandomReachablePointinRadius (Variables|GhostForm|GetGhostFormHomeLocation) (Variables|GhostForm|GetGhostFormMoveRadius) 0 0)) 0 5.0 false
    (:OnSuccess
      _)
    (:OnFail
      _))
  (CallFunction|StartGhostFormMoveTimer))

(event EventBeginPlay
  (CallFunction|OnEnterGhostForm true)
  (Variables|Default|SetMovementDisabled (Variables|Default|GetMovementStartDisabled)))

(event EventTick
  (params (DeltaSeconds :type Float%20%28single-precision%29))
  (if (Variables|Default|GetIsMortalForm)
    (if (not (Variables|Default|GetMovementDisabled))
      (AI|AIMoveTo self (Transformation|GetActorLocation (CallFunction|GetTSGPlayerPawn)) 0 5.0 false))))

(event EventEnterGhostForm
  (params (EnteringInitialState :type Boolean))
  (CallFunction|OnEnterGhostForm false))

(event EventEnterMortalForm
  (CallFunction|OnEnterMortalForm))

(fn ConstructionScript)

(fn OnEnterGhostForm
  (params (EnteringInitialState :type Boolean))
  (bind _charactermovement (Variables|Character|GetCharacterMovement))
  (Utilities|FlowControl|Sequence
    (:then_0
      (Variables|Default|SetIsMortalForm false))
    (:then_1
      (Rendering|SetVisibility (Variables|Default|GetGuardA_Body_Ghost) true false)
      (Rendering|SetVisibility (Variables|Default|GetGuardA_Body_Real) false false))
    (:then_2
      (Variables|GhostForm|SetGhostFormHomeLocation (Transformation|GetActorLocation))
      (CallFunction|StartGhostFormMoveTimer))
    (:then_3
      (Variables|/Script/Engine.CharacterMovementComponent|SetMaxWalkSpeed _charactermovement (Variables|Default|GetGhostWalkSpeed))
      (Variables|/Script/Engine.CharacterMovementComponent|SetMaxAcceleration _charactermovement (Variables|Default|GetGhostAcceleration))
      (Variables|/Script/Engine.CharacterMovementComponent|SetRotationRate _charactermovement (Math|Rotator|MakeRotator 0.0 0.0 (Variables|Default|GetGhostRotationRate))))))

(fn OnEnterMortalForm
  (bind _charactermovement (Variables|Character|GetCharacterMovement))
  (Utilities|FlowControl|Sequence
    (:then_0
      (Variables|Default|SetIsMortalForm true))
    (:then_1
      (Rendering|SetVisibility (Variables|Default|GetGuardA_Body_Ghost) false false)
      (Rendering|SetVisibility (Variables|Default|GetGuardA_Body_Real) true false))
    (:then_2
      (Utilities|Time|ClearandInvalidateTimerbyHandle (Variables|GhostForm|GetGhostFormRandomMoveTimer)))
    (:then_3
      (Variables|/Script/Engine.CharacterMovementComponent|SetMaxWalkSpeed _charactermovement (Variables|Default|GetMortalWalkSpeed))
      (Variables|/Script/Engine.CharacterMovementComponent|SetMaxAcceleration _charactermovement (Variables|Default|GetMortalAcceleration))
      (Variables|/Script/Engine.CharacterMovementComponent|SetRotationRate _charactermovement (Math|Rotator|MakeRotator 0.0 0.0 (Variables|Default|GetMortalRotationRate))))))

(fn StartGhostFormMoveTimer
  (bind _returnvalue (Utilities|Time|SetTimerbyEvent (EventDispatchers|CreateEvent :!event Custom|GhostFormMoveEvent) (Math|Random|RandomFloatinRange (Variables|GhostForm|GetGhostFormMoveMinTime) (Variables|GhostForm|GetGhostFormMoveMaxTime))))
  (Variables|GhostForm|SetGhostFormRandomMoveTimer _returnvalue))

(fn AllowMovement
  (params (Bool :type Boolean))
  (Variables|Default|SetMovementDisabled (not Bool)))