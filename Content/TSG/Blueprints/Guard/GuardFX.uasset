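; GuardFX is a guard effects Blueprint that plays a repeating cry sound attached to itself, varying with the player's mortal or ghost form.
; From BeginPlay, an endless delay loop spawns CryCue with randomized timing and pitch.
; Mortal form gives shorter gaps and raised pitch; otherwise cries are less frequent and much deeper.
; The form is polled through IsPlayerMortalForm, while the EnterGhostForm and EnterMortalForm events are empty.
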(event EventBeginPlay
  (bind _bool (CallFunction|IsPlayerMortalForm))
  (Utilities|FlowControl|Delay (select _bool (Math|Random|RandomFloatinRange 0.3 2.0) (Math|Random|RandomFloatinRange 1.0 3.0)) :!label _label)
  (Audio|SpawnSoundAttached (Variables|Default|GetCryCue) self "None" "0, 0, 0" "0, 0, 0" "KeepRelativeOffset" false 2.0 (select _bool (Math|Random|RandomFloatinRange 1.0 2.0) (Math|Random|RandomFloatinRange 0.1 0.5)) 0.0 0 0)
  (goto _label))

(event EventTick
  (params (DeltaSeconds :type Float%20%28single-precision%29)))

(event EventEnterGhostForm
  (params (EnteringInitialState :type Boolean)))

(event EventEnterMortalForm)